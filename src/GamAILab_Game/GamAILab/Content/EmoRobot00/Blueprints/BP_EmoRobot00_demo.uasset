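; Demo actor for the EmoRobot character, with configurable look, emotion and looping animation.
; The construction script shows either the mouth or the speech mesh and builds dynamic materials for body, eyes, mouth and speech from exposed color, glow, decal and emotion settings.
; BeginPlay loops the chosen animation.
; When RainbowDance is on, Tick cycles only the body's emission color using three phase-shifted sine waves.
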(event `self.ReceiveBeginPlay`
  (`SkeletalMeshComponent.PlayAnimation` (`self.Robot`) (`self.AnimationSet`) true))

(event `self.ReceiveTick`
  (params (DeltaSeconds :type "Float (single-precision)"))
  (if (`self.RainbowDance`)
    (bind _output_get (set `self.RainBowTime` (+ (`self.RainBowTime`) (* (`self.RainbowSpeed`) DeltaSeconds))))
    (`MaterialInstanceDynamic.SetVectorParameterValue` (`self.MID_Robot`) "Emission Color" (make `LinearColor` (* (`KismetMathLibrary.Sin` _output_get) 0.5) (* (`KismetMathLibrary.Sin` (+ _output_get 2.094)) 0.5) (* (`KismetMathLibrary.Sin` (+ _output_get 4.188)) 0.5) 1.0))))

(fn `UserConstructionScript`
  (bind _mid_robot (`self.MID_Robot`))
  (bind _mouthspeak (`self.MouthSpeak`))
  (bind _emission_power (`self.Emission Power`))
  (bind _glowcolor (`self.GlowColor`))
  (bind _returnvalue (`KismetMathLibrary.Conv_IntToDouble` (+ (`self.Emotion Index`) -1)))
  (`SceneComponent.SetVisibility` (`self.Mouth`) (not _mouthspeak) false)
  (`SceneComponent.SetVisibility` (`self.Speach`) _mouthspeak false)
  (bind _returnvalue_2 (`PrimitiveComponent.CreateDynamicMaterialInstance` (`self.Robot`) 0 "/Game/EmoRobot00/Materials/MI_EmoRobot00a.MI_EmoRobot00a" "None"))
  (set `self.MID_Robot` _returnvalue_2)
  (`MaterialInstanceDynamic.SetVectorParameterValue` _mid_robot "Emission Color" _glowcolor)
  (`MaterialInstanceDynamic.SetScalarParameterValue` _mid_robot "Emission Power" _emission_power)
  (`MaterialInstanceDynamic.SetVectorParameterValue` _mid_robot "Body Color" (`self.Body color`))
  (`MaterialInstanceDynamic.SetVectorParameterValue` _mid_robot "Decals Color" (`self.Decals color`))
  (`MaterialInstanceDynamic.SetScalarParameterValue` _mid_robot "Metallic" (`self.Metallic`))
  (`MaterialInstanceDynamic.SetTextureParameterValue` _mid_robot "Decals" (`self.Decals`))
  (`MaterialInstanceDynamic.SetScalarParameterValue` _mid_robot "Tiling X" (`self.Tiling_X`))
  (`MaterialInstanceDynamic.SetScalarParameterValue` _mid_robot "Tiling Y" (`self.Tililng_Y`))
  (bind _returnvalue_3 (`PrimitiveComponent.CreateDynamicMaterialInstance` (`self.Eyes`) 0 "/Game/EmoRobot00/Materials/MI_Emotions.MI_Emotions" "None"))
  (`MaterialInstanceDynamic.SetVectorParameterValue` _returnvalue_3 "Emission Color" _glowcolor)
  (`MaterialInstanceDynamic.SetScalarParameterValue` _returnvalue_3 "Emission Power" _emission_power)
  (`MaterialInstanceDynamic.SetScalarParameterValue` _returnvalue_3 "Emotion index" _returnvalue)
  (bind _returnvalue_4 (`PrimitiveComponent.CreateDynamicMaterialInstance` (`self.Mouth`) 0 "/Game/EmoRobot00/Materials/MI_Emotions.MI_Emotions" "None"))
  (`MaterialInstanceDynamic.SetVectorParameterValue` _returnvalue_4 "Emission Color" _glowcolor)
  (`MaterialInstanceDynamic.SetScalarParameterValue` _returnvalue_4 "Emission Power" _emission_power)
  (`MaterialInstanceDynamic.SetScalarParameterValue` _returnvalue_4 "Emotion index" _returnvalue)
  (bind _returnvalue_5 (`PrimitiveComponent.CreateDynamicMaterialInstance` (`self.Speach`) 0 "/Game/EmoRobot00/Materials/MI_Speach.MI_Speach" "None"))
  (`MaterialInstanceDynamic.SetVectorParameterValue` _returnvalue_5 "Emission Color" _glowcolor)
  (`MaterialInstanceDynamic.SetScalarParameterValue` _returnvalue_5 "Emission Power" _emission_power))